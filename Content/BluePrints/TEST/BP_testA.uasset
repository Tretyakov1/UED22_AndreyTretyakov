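; BP_testA is a test actor that displays a name through a TextRender component.
; The construction script sets the text to "My name is" followed by MyName, and BeginPlay keeps it visible only when MyName is "bob".
; Tick prints the delta time and a "Hello World" message on screen each frame, while some leftover print, delay and variable nodes are never executed.
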(event `self.ReceiveBeginPlay`
  (`SceneComponent.SetVisibility` (`self.TextRender`) (== (`self.MyName`) "bob") false))

(event `self.ReceiveTick`
  (params (DeltaSeconds :type "Float (single-precision)"))
  (`KismetSystemLibrary.PrintString` (`KismetStringLibrary.Conv_DoubleToString` DeltaSeconds) true false (struct :`G` 0.66 :`B` 1.0 :`A` 1.0) DeltaSeconds)
  (`KismetSystemLibrary.PrintString` " Hello World" true false (struct :`R` 0.75 :`G` 0.314893 :`B` 0.526895 :`A` 1.0) DeltaSeconds))

(fn `UserConstructionScript`
  (`TextRenderComponent.K2_SetText` (`self.TextRender`) (`|FormatText` "My name is {Name}" (`self.MyName`))))