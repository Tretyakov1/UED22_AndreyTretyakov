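; BP_Door_WithLock is a child door that opens only while unlocked, with a point light showing red for locked and green for unlocked.
; Interact toggles an unlocked door, or checks the overlapping actor's backpack component for the needed key names on a locked one.
; Matched keys are removed even if the set is incomplete, and the door unlocks only when all are found at once.
; Lock works only on doors without required keys.
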(event `self.OpenDoor`
  (if (not (`self.IsDoorLocked`))
    (`parent.OpenDoor`)))

(event `self.CloseDoor`
  (`parent.CloseDoor`))

(fn `Interact`
  (returns (Success :type Boolean))
  (locals (L_Backpack :type "/Game/BluePrints/Components/BP_BackpackComponent Object Reference") (L_ItemInrement :type Integer) (L_ItemName :type Name))
  (if (`self.IsReadyToInteract`)
    (if (not (`self.IsDoorLocked`))
      (if (`self.IsDoorOpen`)
        (`self.CloseDoor`)
        (return true)
        (else
          (`self.OpenDoor`)))
      (elif (`KismetArrayLibrary.Array_IsValidIndex` (`self.NeededKeysName`))
        (bind _overlappedactor (`self.OverlappedActor`)
          (:`then`
            (bind _returnvalue (`self.GetComponentByClass` _overlappedactor "/Game/BluePrints/Components/BP_BackpackComponent.BP_BackpackComponent_C"))
            (`/Engine/EditorBlueprintResources/StandardMacros.IsValid` _returnvalue
              (:`Is Valid`
                (set `local.L_Backpack` _returnvalue)
                (for _array_element (`self.NeededKeysName`)
                  (set `local.L_ItemName` _array_element)
                  (if (`BlueprintSetLibrary.Set_Contains` (`/Game/BluePrints/Components/BP_BackpackComponent.QuestItems` (`local.L_Backpack`)) (`local.L_ItemName`))
                    (`/Engine/EditorBlueprintResources/StandardMacros.IncrementInt` (`local.L_ItemInrement`)
                      (:`  `
                        ;[0.7927 0.2601 0.3783] For delete items after use
                        (`BlueprintSetLibrary.Set_Remove` (`/Game/BluePrints/Components/BP_BackpackComponent.QuestItems` (`local.L_Backpack`)) (`local.L_ItemName`))))))
                ;[1 1 1] All key ?
                (if (== (`local.L_ItemInrement`) (`KismetArrayLibrary.Array_Length` (`self.NeededKeysName`)))
                  (`self.Unlock`)
                  (else
                    (return true))))
              (:`Is Not Valid`
                (return true))))
          (:`else`
            (return true)))
        (else
          (return true))))
    (else
      (return false))))

(fn `Lock`
  (if (not (`KismetArrayLibrary.Array_IsValidIndex` (`self.NeededKeysName`)))
    (set `self.IsDoorLocked` true)
    (`self.UpdateDoorLockIndication`)))

(fn `SwitchLock`
  (set `self.IsDoorLocked` (not (`self.IsDoorLocked`)))
  (`self.UpdateDoorLockIndication`))

(fn `Unlock`
  (set `self.IsDoorLocked` false)
  (`self.UpdateDoorLockIndication`))

(fn `UpdateDoorLockIndication`
  (`LightComponent.SetLightColor` (`self.PointLightLockIndicator`) (`KismetMathLibrary.SelectColor` (struct :`R` 1.0 :`A` 1.0) (struct :`R` 0.106133 :`G` 0.966667 :`B` 0.23544 :`A` 1.0) (`self.IsDoorLocked`)) true))

(fn `UserConstructionScript`
  (`parent.UserConstructionScript`)
  (`self.UpdateDoorLockIndication`))